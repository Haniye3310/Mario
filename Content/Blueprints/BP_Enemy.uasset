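; BP_Enemy is a side-scrolling patrol enemy for a Mario-style game, moving along its local X axis each Tick by Speed and Direction.
; Its Box overlap destroys BP_Mario and restarts player 0 through the GameMode, while any other overlap flips Direction to turn it around.
; An overlap of Mario with the Head component swaps the Sprite to a death flipbook, then destroys the enemy after a short delay.
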(event `self.ReceiveTick`
  (params (DeltaSeconds :type "Float (single-precision)"))
  (`self.K2_AddActorLocalOffset` (`KismetMathLibrary.MakeVector` (* (* DeltaSeconds (`self.Direction`)) (`self.Speed`)))))

(event `self.Box.OnComponentBeginOverlap`
  (params (OverlappedComponent :type "PrimitiveComponent Object Reference") (OtherActor :type "Actor Object Reference") (OtherComp :type "PrimitiveComponent Object Reference") (OtherBodyIndex :type Integer) (bFromSweep :type Boolean) (SweepResult :type "HitResult Structure (by ref)"))
  (bind _asbp_mario (cast `/Game/Blueprints/BP_Mario` OtherActor)
    (:`then`
      (`self.K2_DestroyActor` _asbp_mario)
      (`GameModeBase.RestartPlayer` (`GameplayStatics.GetGameMode`) (`GameplayStatics.GetPlayerController` 0)))
    (:`CastFailed`
      (set `self.Direction` (* (`self.Direction`) -1.0)))))

(event `self.Head.OnComponentBeginOverlap`
  (params (OverlappedComponent :type "PrimitiveComponent Object Reference") (OtherActor :type "Actor Object Reference") (OtherComp :type "PrimitiveComponent Object Reference") (OtherBodyIndex :type Integer) (bFromSweep :type Boolean) (SweepResult :type "HitResult Structure (by ref)"))
  (cast `/Game/Blueprints/BP_Mario` OtherActor)
  (`PaperFlipbookComponent.SetFlipbook` (`self.Sprite`) "/Game/Sprites/FB_Enemy_Death.FB_Enemy_Death")
  (`KismetSystemLibrary.Delay` 0.2)
  (`self.K2_DestroyActor`))

(fn `UserConstructionScript`)