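; BP_Mario is the side-scrolling player character, with Enhanced Input for moving along world X and jumping.
; Movement input also snaps control rotation yaw between 0 and 180 to set facing.
; Each tick, while the BP_Camera found at BeginPlay is valid, it drags that camera along X only and picks the idle, run or jump flipbook.
; The node setting that camera as view target is left unconnected.
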(event `self.ReceiveBeginPlay`
  (`EnhancedInputSubsystemInterface.AddMappingContext` (pcsubsystem `EnhancedInputLocalPlayerSubsystem` (`GameplayStatics.GetPlayerController` 0)) "/Game/Input/MC_Mario.MC_Mario" 0 (struct))
  (bind _returnvalue (`GameplayStatics.GetActorOfClass` "/Game/Blueprints/BP_Camera.BP_Camera_C"))
  (bind _output_get (set `self.CameraRef` _returnvalue)))

(event `self.ReceiveTick`
  (params (DeltaSeconds :type "Float (single-precision)"))
  (bind _returnvalue_x (`KismetMathLibrary.BreakVector` (`self.K2_GetActorLocation`)))
  (bind _returnvalue_x_2 (`KismetMathLibrary.BreakVector` (`self.GetVelocity`)))
  (bind _cameraref (`self.CameraRef`)
    (:`then`
      (bind (_returnvalue_x_3 _returnvalue_y _returnvalue_z) (`KismetMathLibrary.BreakVector` (`self.K2_GetActorLocation` _cameraref)))
      (`self.K2_SetActorLocation` _cameraref (`KismetMathLibrary.MakeVector` _returnvalue_x _returnvalue_y _returnvalue_z) false false)
      (if (`NavMovementInterface.IsMovingOnGround` (`self.CharacterMovement`))
        (`PaperFlipbookComponent.SetFlipbook` (`self.Sprite`) (select `bool` (> (`KismetMathLibrary.Abs` _returnvalue_x_2) 0.0) :`false` "/Game/Sprites/Flipbooks/Flipbook_Idle.Flipbook_Idle" :`true` "/Game/Sprites/Flipbooks/Flipbook_Run.Flipbook_Run" :!type "PaperFlipbook Object Reference"))
        (else
          (`PaperFlipbookComponent.SetFlipbook` (`self.Sprite`) "/Game/Sprites/Flipbooks/Flipbook_Jump.Flipbook_Jump"))))
    (:`else`)))

(event `EnhancedInput|/Game/Input/Jump`
  (params (ActionValue :type Boolean) (ElapsedSeconds :type "Float (double-precision)") (TriggeredSeconds :type "Float (double-precision)") (InputAction :type "InputAction Object Reference" :default "/Game/Input/Jump.Jump"))
  (:`Started`
    (`self.Jump`))
  (:`Completed`
    (`self.StopJumping`)))

(event `EnhancedInput|/Game/Input/Move`
  (params (ActionValue :type "Float (double-precision)") (ElapsedSeconds :type "Float (double-precision)") (TriggeredSeconds :type "Float (double-precision)") (InputAction :type "InputAction Object Reference" :default "/Game/Input/Move.Move"))
  (:`Triggered`
    (`self.AddMovementInput` (1.0 0.0 0.0) ActionValue)
    (`Controller.SetControlRotation` (`self.GetController`) (`KismetMathLibrary.MakeRotator` 0.0 0.0 (select `bool` (> ActionValue 0.0) :`false` 180.0)))))

(fn `UserConstructionScript`)