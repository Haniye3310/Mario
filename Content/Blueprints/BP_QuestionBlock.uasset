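; BP_QuestionBlock is a Paper2D question block that gives BP_Mario coins when he overlaps its Box1 trigger.
; The overlap plays a timeline that offsets the block sprite from its starting height and moves the coin vertically.
; Timeline updates also set the block's flipbook and make the trigger ignore all channels, preventing further hits.
; When the timeline finishes, the coin component is destroyed and CoinValue is added to Mario's coin count.
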(event `self.Box1.OnComponentBeginOverlap`
  (params (OverlappedComponent :type "PrimitiveComponent Object Reference") (OtherActor :type "Actor Object Reference") (OtherComp :type "PrimitiveComponent Object Reference") (OtherBodyIndex :type Integer) (bFromSweep :type Boolean) (SweepResult :type "HitResult Structure (by ref)"))
  (bind _as_bp_mario (`self.As BP Mario`))
  (bind (_relativelocation_x _relativelocation_y _relativelocation_z) (`KismetMathLibrary.BreakVector` (`SceneComponent.RelativeLocation` (`self.RenderComponent`))))
  (bind (_relativelocation_x_2 _relativelocation_y_2) (`KismetMathLibrary.BreakVector` (`SceneComponent.RelativeLocation` (`self.RenderComponent`))))
  (bind _asbp_mario (cast `/Game/Blueprints/BP_Mario` OtherActor))
  (set `self.As BP Mario` _asbp_mario)
  (bind _output_get (set `self.Relative Location Z` _relativelocation_z))
  (bind (_direction _zoffset _coinoffset) (`Timeline|Timeline` :!via `PlayFromStart`)
    (:`Update`
      (`SceneComponent.K2_SetRelativeLocation` (`self.Coin`) (`KismetMathLibrary.MakeVector` 0.0 0.0 _coinoffset) false false)
      (`SceneComponent.K2_SetRelativeLocation` (`self.RenderComponent`) (`KismetMathLibrary.MakeVector` _relativelocation_x_2 _relativelocation_y_2 (+ _zoffset _output_get)) false false)
      (`PrimitiveComponent.SetCollisionResponseToAllChannels` (`self.Box1`) "ECR_Ignore")
      (`PaperFlipbookComponent.SetFlipbook` (`self.RenderComponent`) "/Game/Sprites/FB_QuestionBlock.FB_QuestionBlock"))
    (:`Finished`
      (`ActorComponent.K2_DestroyComponent` (`self.Coin`))
      (set `/Game/Blueprints/BP_Mario.Coin` (+ (`/Game/Blueprints/BP_Mario.Coin` _as_bp_mario) (`self.CoinValue`)) _as_bp_mario))))

(fn `UserConstructionScript`)