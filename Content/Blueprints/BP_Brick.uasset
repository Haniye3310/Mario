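; BP_Brick is a brick block that does a bump animation when BP_Mario overlaps its Box1 trigger.
; The overlap stores the render component's relative Z, then a timeline adds its ZOffset to that height each update while X and Y stay as they are.
; Box1 ignores all channels while the timeline plays and returns to overlap when it finishes, blocking retriggers mid-animation.
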(event `self.Box1.OnComponentBeginOverlap`
  (params (OverlappedComponent :type "PrimitiveComponent Object Reference") (OtherActor :type "Actor Object Reference") (OtherComp :type "PrimitiveComponent Object Reference") (OtherBodyIndex :type Integer) (bFromSweep :type Boolean) (SweepResult :type "HitResult Structure (by ref)"))
  (bind (_relativelocation_x _relativelocation_y _relativelocation_z) (`KismetMathLibrary.BreakVector` (`SceneComponent.RelativeLocation` (`self.RenderComponent`))))
  (bind (_relativelocation_x_2 _relativelocation_y_2) (`KismetMathLibrary.BreakVector` (`SceneComponent.RelativeLocation` (`self.RenderComponent`))))
  (cast `/Game/Blueprints/BP_Mario` OtherActor)
  (bind _output_get (set `self.Relative Location Z` _relativelocation_z))
  (bind (_direction _zoffset) (`Timeline|Timeline` :!via `PlayFromStart`)
    (:`Update`
      (`SceneComponent.K2_SetRelativeLocation` (`self.RenderComponent`) (`KismetMathLibrary.MakeVector` _relativelocation_x_2 _relativelocation_y_2 (+ _zoffset _output_get)) false false)
      (`PrimitiveComponent.SetCollisionResponseToAllChannels` (`self.Box1`) "ECR_Ignore"))
    (:`Finished`
      (`PrimitiveComponent.SetCollisionResponseToAllChannels` (`self.Box1`) "ECR_Overlap"))))

(fn `UserConstructionScript`)